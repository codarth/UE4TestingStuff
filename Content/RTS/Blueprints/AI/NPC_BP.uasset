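; RTS NPC character that randomizes its sex, body color and name on construction and owns a personal HUD widget.
; BeginPlay binds to the camera controller's HUD requests and to GameState speed updates, which recompute walk speed.
; A HUD request locks input to UI, timeline-lerps the camera pawn to the NPC, then opens a Tick gate that follows it in XY.
; SetIsBusy writes the busy flag to the AI blackboard.
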(event Custom|DisplayHUD
  (params (Actor :type Actor%20Object%20Reference))
  (bind _cameracontroller_ref (Variables|References|GetCameraController_REF))
  ;[1 1 1] Display HUD
  (if (and (== Actor self) (not (Variables|Rendering|GetbHidden)))
    (UserInterface|Viewport|AddtoViewport (Variables|Default|GetNPC_HUD) 0)
    (Input|SetInputModeUIOnly _cameracontroller_ref 0 "DoNotLock")
    (Widget|SetIsEnabled (Variables|/Game/RTS/Blueprints/CameraPawnController.CameraPawnController_C|GetMainHUD_REF _cameracontroller_ref) false)
    (bind _newlocation (|LerpLocation)
      (:Update
        (Transformation|SetActorLocation (Variables|/Game/RTS/Blueprints/CameraPawnController.CameraPawnController_C|GetCameraPawn_REF (Variables|References|GetCameraController_REF)) _newlocation false false))
      (:Finished
        (Variables|/Game/RTS/Blueprints/CameraPawnController.CameraPawnController_C|SetDisableCamNav (Variables|References|GetCameraController_REF) true)
        (CallFunction|OpenFollowGate)))))

(event Custom|OpenFollowGate
  (bind _returnvalue (Transformation|GetActorLocation))
  (bind _cameracontroller_ref (Variables|References|GetCameraController_REF))
  (bind _camerapawn_ref (Variables|/Game/RTS/Blueprints/CameraPawnController.CameraPawnController_C|GetCameraPawn_REF _cameracontroller_ref))
  ;[1 1 1] Tick
  (Utilities|FlowControl|Gate true) ; enters at Open
)

(event Custom|CloseFollowGate
  (bind _returnvalue (Transformation|GetActorLocation))
  (bind _cameracontroller_ref (Variables|References|GetCameraController_REF))
  (bind _camerapawn_ref (Variables|/Game/RTS/Blueprints/CameraPawnController.CameraPawnController_C|GetCameraPawn_REF _cameracontroller_ref))
  ;[1 1 1] Tick
  (Utilities|FlowControl|Gate true) ; enters at Close
)

(event Custom|UpdateWalkSpeed
  (params (TimeUnit :type Float%20%28single-precision%29))
  ;[1 1 1] Walk Speed
  (Variables|/Script/Engine.CharacterMovementComponent|SetMaxWalkSpeed (Variables|Character|GetCharacterMovement) (/ (Variables|Default|GetBaseWalkSpeed) (Variables|/Game/RTS/GameBPs/RTSGameState.RTSGameState_C|GetSpeedMultiplier (Variables|References|GetGameState_REF)))))

(event EventBeginPlay
  ;[1 1 1] BeginPlay
  (Variables|References|SetAIController_REF (.AsNPC%20AIController (Utilities|Casting|CastToNPC_AIController (AI|GetAIController self))))
  (bind _ascamera_pawn_controller (Utilities|Casting|CastToCameraPawnController (Game|GetPlayerController 0)))
  (bind _output_get (Variables|References|SetCameraController_REF _ascamera_pawn_controller))
  (EventDispatchers|BindEventtoHUDRequest _output_get (EventDispatchers|CreateEvent :!event Custom|DisplayHUD))
  (bind _returnvalue (UserInterface|CreateWidget "/Game/RTS/HUD/NPC_HUD.NPC_HUD_C" 0 self))
  (Variables|Default|SetNPC_HUD _returnvalue)
  (EventDispatchers|BindEventtoUpdateGameSpeed (Variables|References|GetGameState_REF) (EventDispatchers|CreateEvent :!event Custom|UpdateWalkSpeed))
  (CallFunction|UpdateWalkSpeed 0.0))

(event EventTick
  (params (DeltaSeconds :type Float%20%28single-precision%29))
  (bind _returnvalue (Transformation|GetActorLocation))
  (bind _cameracontroller_ref (Variables|References|GetCameraController_REF))
  (bind _camerapawn_ref (Variables|/Game/RTS/Blueprints/CameraPawnController.CameraPawnController_C|GetCameraPawn_REF _cameracontroller_ref))
  ;[1 1 1] Tick
  (Utilities|FlowControl|Gate true
    (:Exit
      (Transformation|SetActorLocation _camerapawn_ref (Math|Vector|MakeVector (.x _returnvalue) (.y _returnvalue) (.z (Transformation|GetActorLocation _camerapawn_ref))) false false))))

(fn ConstructionScript
  (CallFunction|RandomNPCFeatures))

(fn RandomNPCFeatures
  (bind _returnvalue (Rendering|Material|CreateDynamicMaterialInstance (Variables|Character|GetMesh) 0 "/Game/Mannequin/Character/Materials/M_UE4Man_Body_Inst.M_UE4Man_Body_Inst" "None" :!class /Script/Engine.PrimitiveComponent))
  (LocalVariables|SetMaterialInstance _returnvalue)
  (switch int (Math|Random|RandomIntegerinRange 0 (- (|GetNumEnumEntries) 1))
    (:0
      (Rendering|Material|SetVectorParameterValue (LocalVariables|GetMaterialInstance) "BodyColor" (LocalVariables|GetMaleColor) :!class /Script/Engine.MaterialInstanceDynamic)
      (bind _name (CallFunction|GetRandomName "NewEnumerator0"))
      (Variables|Default|SetMyProfile (Utilities|Struct|MakeNPC_Profile_Struct _name "NewEnumerator0")))
    (:1
      (Rendering|Material|SetVectorParameterValue (LocalVariables|GetMaterialInstance) "BodyColor" (LocalVariables|GetFemaleColor) :!class /Script/Engine.MaterialInstanceDynamic)
      (bind _name_2 (CallFunction|GetRandomName "NewEnumerator1"))
      (Variables|Default|SetMyProfile (Utilities|Struct|MakeNPC_Profile_Struct _name_2 "NewEnumerator1")))))

(fn GetRandomName
  (params (Sex :type NPC_Sex_ENUM%20Enum :default "NewEnumerator0"))
  (bind _returnvalue (|GetNumEnumEntries))
  (bind _returnvalue_2 (|GetNumEnumEntries))
  (bind _returnvalue_3 (- _returnvalue_2 1))
  (bind _returnvalue_4 (- _returnvalue 1))
  (bind _returnvalue_5 (Math|Random|RandomIntegerinRange 0 _returnvalue_3))
  (bind _returnvalue_6 (Math|Random|RandomIntegerinRange 0 _returnvalue_4))
  (bind _returnvalue_7 (Math|Conversions|ToByte(Integer) _returnvalue_5))
  (bind _returnvalue_8 (Math|Conversions|ToByte(Integer) _returnvalue_6))
  (bind _returnvalue_9 (Utilities|Enum|ByteToEnumNPC_NameMale_ENUM _returnvalue_8))
  (bind _returnvalue_10 (Utilities|Enum|ByteToEnumNPC_NameFemale_ENUM _returnvalue_7))
  (bind _returnvalue_11 (Utilities|Enum|LiteralenumNPC_NameMale_ENUM _returnvalue_9))
  (bind _returnvalue_12 (Utilities|Enum|LiteralenumNPC_NameFemale_ENUM _returnvalue_10))
  (if (Utilities|Enum|Equal(Enum) Sex "NewEnumerator0")
    (Development|PrintString (Utilities|String|Append "Number of names: " (Utilities|String|ToString(Integer) _returnvalue) "   -1: " (Utilities|String|ToString(Integer) _returnvalue_4) "   Ramdon#: " (Utilities|String|ToString(Integer) _returnvalue_6) "   toByte: " (Utilities|String|ToString(Byte) _returnvalue_8) "   Afterbyte: " (Utilities|String|EnumtoString _returnvalue_9) "   Enum Value: " (Utilities|String|EnumtoString _returnvalue_11)) true true "(R=0.000000,G=0.660000,B=1.000000,A=1.000000)" 1e+01)
    (return (Utilities|String|EnumtoString _returnvalue_11))
    (else
      (Development|PrintString (Utilities|String|Append "Number of names: " (Utilities|String|ToString(Integer) _returnvalue_2) "   -1: " (Utilities|String|ToString(Integer) _returnvalue_3) "   Ramdon#: " (Utilities|String|ToString(Integer) _returnvalue_5) "   toByte: " (Utilities|String|ToString(Byte) _returnvalue_7) "   Afterbyte: " (Utilities|String|EnumtoString _returnvalue_10) "   Enum Value: " (Utilities|String|EnumtoString _returnvalue_12)) true true "(R=0.000000,G=0.660000,B=1.000000,A=1.000000)" 1e+01)
      (return (Utilities|String|EnumtoString _returnvalue_12)))))

(fn SetIsBusy
  (params (IsBusy :type Boolean))
  (AI|Components|Blackboard|SetValueasBool (AI|GetBlackboard (Variables|References|GetAIController_REF)) (Variables|Default|GetIsBusy) IsBusy)
  (return))