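; RTS player controller that drives the camera pawn, object selection and building placement.
; On BeginPlay it spawns the construction manager and ghost building, then creates the main HUD.
; Camera supports zoom-scaled axis movement, screen-edge scrolling, gated mouse rotation and spring-arm zoom.
; In build mode the ghost follows the cursor, rotates and queues construction on valid clicks; otherwise clicks send selections to the HUD, and V spawns an NPC.
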(event EventBeginPlay
  (bind _returnvalue (Math|Transform|MakeTransform "0, 0, 0" "0, 0, 0" "0.500000,0.500000,0.500000"))
  ;[1 1 1] Begin PLay
  (Utilities|FlowControl|Sequence
    (:then_0
      (Utilities|ReferenceCasts))
    (:then_1
      (bind _returnvalue_2 (Game|SpawnActorfromClass "/Game/RTS/Blueprints/Construction/ConstructionManager_BP.ConstructionManager_BP_C" _returnvalue "AlwaysSpawn" 0 0))
      (Variables|References|SetConstructionManager_REF _returnvalue_2))
    (:then_2
      (bind _returnvalue_3 (Game|SpawnActorfromClass "/Game/RTS/Blueprints/Buildings/GhostBuilding_BP.GhostBuilding_BP_C" _returnvalue "AlwaysSpawn" 0 self 0))
      (Variables|References|SetGhostBuilding_REF _returnvalue_3))
    (:then_3
      (Input|SetInputModeGameandUI self 0 "LockAlways" true)
      (Utilities|CreateHUD)
      (UserInterface|Viewport|AddtoViewport (Variables|References|GetMainHUD_REF) 0))))

(event EventTick
  (params (DeltaSeconds :type Float%20%28single-precision%29))
  (if (Variables|Default|GetBuildModeActive)
    (|SetCursorWolrdPosition)))

(event Input|ActionEvents|InputActionPan
  (params (Key :type Key%20Structure))
  (bind _camerapawn_ref (Variables|References|GetCameraPawn_REF))
  (bind _returnvalue (Transformation|GetActorRotation _camerapawn_ref))
  (bind (_roll _pitch _yaw) (Math|Rotator|BreakRotator _returnvalue))
  ;[1 1 1] CameraMovement
  ;;[1 1 1] Pan Y
  (:Pressed
    (Variables|Default|SetDisableCamNav true)
    (Utilities|FlowControl|Gate true) ; enters at Open
  )
  (:Released
    (Variables|Default|SetDisableCamNav false)
    (Utilities|FlowControl|Gate true) ; enters at Close
  ))

(event Input|ActionEvents|InputActionPan
  (params (Key :type Key%20Structure))
  (bind _camerapawn_ref (Variables|References|GetCameraPawn_REF))
  (bind _returnvalue (Transformation|GetActorRotation _camerapawn_ref))
  (bind (_roll _pitch _yaw) (Math|Rotator|BreakRotator _returnvalue))
  ;[1 1 1] CameraMovement
  ;;[1 1 1] Pan X
  (:Pressed
    (Variables|Default|SetDisableCamNav true)
    (Utilities|FlowControl|Gate true) ; enters at Open
  )
  (:Released
    (Variables|Default|SetDisableCamNav false)
    (Utilities|FlowControl|Gate true) ; enters at Close
  ))

(event Input|ActionEvents|InputActionPanReset
  (params (Key :type Key%20Structure))
  (bind _camerapawn_ref (Variables|References|GetCameraPawn_REF))
  (bind _returnvalue (Transformation|GetActorRotation _camerapawn_ref))
  (bind (_roll _pitch _yaw) (Math|Rotator|BreakRotator _returnvalue))
  ;[1 1 1] CameraMovement
  ;;[1 1 1] Pan Reset
  (:Pressed
    (Transformation|SetActorRotation _camerapawn_ref (Math|Rotator|MakeRotator _roll 0.0 _yaw))))

(event Input|ActionEvents|InputActionZoomIn
  (params (Key :type Key%20Structure))
  (bind _camerapawn_ref (Variables|References|GetCameraPawn_REF))
  (bind _springarm (Variables|/Game/RTS/Blueprints/CameraPawn.CameraPawn_C|GetSpringArm _camerapawn_ref))
  ;[1 1 1] CameraMovement
  ;;[1 1 1] Zoom
  (:Pressed
    (Variables|/Script/Engine.SpringArmComponent|SetTargetArmLength _springarm (Math|Float|Clamp(Float) (- (Variables|/Script/Engine.SpringArmComponent|GetTargetArmLength _springarm) (Variables|Default|GetZoomSensitivity)) 1e+03 (Variables|Default|GetMaxArmDistance)))))

(event Input|ActionEvents|InputActionZoomOut
  (params (Key :type Key%20Structure))
  (bind _camerapawn_ref (Variables|References|GetCameraPawn_REF))
  (bind _springarm (Variables|/Game/RTS/Blueprints/CameraPawn.CameraPawn_C|GetSpringArm _camerapawn_ref))
  ;[1 1 1] CameraMovement
  ;;[1 1 1] Zoom
  (:Pressed
    (Variables|/Script/Engine.SpringArmComponent|SetTargetArmLength _springarm (Math|Float|Clamp(Float) (+ (Variables|Default|GetZoomSensitivity) (Variables|/Script/Engine.SpringArmComponent|GetTargetArmLength _springarm)) 1e+03 (Variables|Default|GetMaxArmDistance)))))

(event Input|ActionEvents|InputActionZoomReset
  (params (Key :type Key%20Structure))
  ;[1 1 1] CameraMovement
  ;;[1 1 1] Zoom Reset
  (:Pressed
    (Variables|/Script/Engine.SpringArmComponent|SetTargetArmLength (Variables|/Game/RTS/Blueprints/CameraPawn.CameraPawn_C|GetSpringArm (Variables|References|GetCameraPawn_REF)) 2.5e+03)))

(event Input|ActionEvents|InputActionDeselect
  (params (Key :type Key%20Structure))
  (:Pressed
    (if (Variables|Default|GetBuildModeActive)
      (Default|KillGhost (Variables|References|GetGhostBuilding_REF))
      (Variables|Default|SetBuildModeActive false))))

(event Input|ActionEvents|InputActionRotateBuildingRight
  (params (Key :type Key%20Structure))
  (bind _ghostbuilding_ref (Variables|References|GetGhostBuilding_REF))
  (bind _returnvalue (Transformation|GetActorRotation _ghostbuilding_ref))
  (bind (_roll _pitch _yaw) (Math|Rotator|BreakRotator _returnvalue))
  (:Pressed
    (if (and (Utilities|IsValid _ghostbuilding_ref) (Variables|Default|GetBuildModeActive))
      (Transformation|SetActorRotation _ghostbuilding_ref (Math|Rotator|MakeRotator _roll _pitch (- _yaw (Variables|Default|GetBuildingRotationRate)))))))

(event Input|ActionEvents|InputActionRotateBuildingLeft
  (params (Key :type Key%20Structure))
  (bind _ghostbuilding_ref (Variables|References|GetGhostBuilding_REF))
  (bind _returnvalue (Transformation|GetActorRotation _ghostbuilding_ref))
  (bind (_roll _pitch _yaw) (Math|Rotator|BreakRotator _returnvalue))
  (:Pressed
    (if (and (Utilities|IsValid _ghostbuilding_ref) (Variables|Default|GetBuildModeActive))
      (Transformation|SetActorRotation _ghostbuilding_ref (Math|Rotator|MakeRotator _roll _pitch (+ _yaw (Variables|Default|GetBuildingRotationRate)))))))

(event Input|AxisEvents|InputAxisMoveForward
  (params (AxisValue :type Float%20%28single-precision%29))
  (bind _camerapawn_ref (Variables|References|GetCameraPawn_REF))
  ;[1 1 1] CameraMovement
  ;;[1 1 1] Movement X
  (if (not (Variables|Default|GetDisableCamNav))
    (Transformation|SetActorTransform _camerapawn_ref (Utilities|MovementX (CallFunction|MovementSpeedCalculation) (Variables|Default|GetFastMoveMultiplier) AxisValue _camerapawn_ref))))

(event Input|AxisEvents|InputAxisMoveRight
  (params (AxisValue :type Float%20%28single-precision%29))
  (bind _movesensativity (CallFunction|MovementSpeedCalculation))
  (bind _fastmovemultiplier (Variables|Default|GetFastMoveMultiplier))
  (bind _camerapawn_ref (Variables|References|GetCameraPawn_REF))
  (bind _transform (Utilities|MovementY AxisValue _movesensativity _fastmovemultiplier _camerapawn_ref))
  (bind (_location _rotation _scale) (Math|Transform|BreakTransform _transform))
  (bind (_x _y) (Math|Vector|BreakVector _location))
  ;[1 1 1] CameraMovement
  ;;[1 1 1] Movement Y
  (if (not (Variables|Default|GetDisableCamNav))
    (Transformation|SetActorTransform _camerapawn_ref (Math|Transform|MakeTransform (Math|Vector|MakeVector _x _y 1.5e+02) _rotation _scale))))

(event Input|MouseEvents|MouseX
  (params (AxisValue :type Float%20%28single-precision%29))
  (bind _camerapawn_ref (Variables|References|GetCameraPawn_REF))
  (bind _returnvalue (Transformation|GetActorRotation _camerapawn_ref))
  (bind (_roll _pitch _yaw) (Math|Rotator|BreakRotator _returnvalue))
  ;[1 1 1] CameraMovement
  ;;[1 1 1] Pan X
  (Utilities|FlowControl|Gate true
    (:Exit
      (Transformation|SetActorRotation (Variables|References|GetCameraPawn_REF) (Math|Rotator|MakeRotator _roll _pitch (+ _yaw (* (Variables|Default|GetPanSensitivity) AxisValue)))))))

(event Input|MouseEvents|MouseY
  (params (AxisValue :type Float%20%28single-precision%29))
  (bind _camerapawn_ref (Variables|References|GetCameraPawn_REF))
  (bind _returnvalue (Transformation|GetActorRotation _camerapawn_ref))
  (bind (_roll _pitch _yaw) (Math|Rotator|BreakRotator _returnvalue))
  ;[1 1 1] CameraMovement
  ;;[1 1 1] Pan Y
  (Utilities|FlowControl|Gate true
    (:Exit
      (Transformation|SetActorRotation (Variables|References|GetCameraPawn_REF) (Math|Rotator|MakeRotator _roll (Math|Float|Clamp(Float) (+ _pitch (* (Variables|Default|GetPanSensitivity) AxisValue)) -15.0 35.0) _yaw)))))

(event Input|MouseEvents|MouseX
  (params (AxisValue :type Float%20%28single-precision%29))
  ;[1 1 1] CameraMovement
  ;;[1 1 1] Edge Movement
  (if (not (Variables|Default|GetDisableCamNav))
    (bind (_deltaxspeed _deltayspeed) (Utilities|ScreenEdgeMovement))
    (Transformation|AddActorLocalOffset (Variables|References|GetCameraPawn_REF) (Math|Vector|MakeVector _deltaxspeed _deltayspeed 0.0) true false)))

(event Input|MouseEvents|MouseY
  (params (AxisValue :type Float%20%28single-precision%29))
  ;[1 1 1] CameraMovement
  ;;[1 1 1] Edge Movement
  (if (not (Variables|Default|GetDisableCamNav))
    (Utilities|ScreenEdgeMovement) ; enters at MouseY
  ))

(event Input|KeyboardEvents|LeftShift
  (params (Key :type Key%20Structure))
  ;[1 1 1] CameraMovement
  ;;[1 1 1] Fast Move
  (:Pressed
    (Variables|Default|SetFastMoveMultiplier 2.0))
  (:Released
    (Variables|Default|SetFastMoveMultiplier 1.0)))

(event Input|MouseEvents|LeftMouseButton
  (params (Key :type Key%20Structure))
  (bind _selectableobjectsenum (Variables|Default|GetSelectableObjectsENUM))
  (bind _hitresult (Class|PlayerController|GetHitResultUnderCursorforObjects _selectableobjectsenum true))
  (bind _hitactor (Collision|BreakHitResult _hitresult))
  (:Pressed
    (if (Variables|Default|GetBuildModeActive)
      (if (|VerifyAsPlaceable)
        (bind _constructionstruct (Default|GetConstructionStruct (Variables|References|GetGhostBuilding_REF)))
        (Default|QueueConstruction (Variables|References|GetConstructionManager_REF) _constructionstruct)
        (Default|KillGhost (Variables|References|GetGhostBuilding_REF)))
      (elif (!= _hitactor 0)
        (Default|CallHUDRequest _hitactor)))))

(event Input|KeyboardEvents|V
  (params (Key :type Key%20Structure))
  (bind _self self)
  (bind _location (CallFunction|SetCursorWorldPosition _self 1e+04))
  (:Pressed
    (Game|SpawnActorfromClass "/Game/RTS/Blueprints/AI/NPC_BP.NPC_BP_C" (Math|Transform|MakeTransform (Math|Vector|MakeVector (.x _location) (.y _location) 1.5e+02) "0, 0, 0" "0.500000,0.500000,0.500000") "Undefined" 0 0)))

(fn ConstructionScript)

(fn MovementSpeedCalculation
  (return (Math|Float|Clamp(Float) (/ (Variables|/Script/Engine.SpringArmComponent|GetTargetArmLength (Variables|/Game/RTS/Blueprints/CameraPawn.CameraPawn_C|GetSpringArm (Variables|References|GetCameraPawn_REF))) 1e+02) 5.0 2e+01)))

(fn SetSightDistance
  (return (+ (Variables|Default|GetSightDistance) (Variables|/Script/Engine.SpringArmComponent|GetTargetArmLength (Variables|/Game/RTS/Blueprints/CameraPawn.CameraPawn_C|GetSpringArm (Variables|References|GetCameraPawn_REF))))))

(fn SetCalandar
  (params (Date :type Array%20of%20Integers))
  (return false))

(fn SetClock
  (params (Time :type Array%20of%20Integers))
  (return false))