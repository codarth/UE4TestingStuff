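; Actor Blueprint that builds a box of cubes one at a time during play, sized by the Size vector.
; On BeginPlay a looping timer fires Builder at the CubesPerSecond rate, adding one instance to an InstancedStaticMesh per tick.
; A running Counter is converted into 100-unit grid coordinates, filling row by row, then layer by layer upward.
; Adding stops at the floored Size volume, though the timer keeps running.
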(event Custom|Builder
  (bind _size (Variables|Default|GetSize))
  (bind _counter (Variables|Default|GetCounter))
  (bind (_x _y _z) (Math|Vector|BreakVector _size))
  (bind _returnvalue (Math|Float|Floor _x))
  (bind _returnvalue_2 (Math|Float|Floor _y))
  (bind _returnvalue_3 (* _returnvalue _returnvalue_2))
  (bind _returnvalue_4 (/ _counter _returnvalue_3))
  (if (<= (Variables|Default|GetCounter) (- (* _returnvalue_3 (Math|Float|Floor _z)) 1))
    (Components|InstancedStaticMesh|AddInstance (Variables|Default|GetInstancedStaticMesh) (Math|Transform|MakeTransform (* (Math|Vector|MakeVector (Math|Conversions|ToFloat(Integer) (- (/ _counter _returnvalue) (* _returnvalue_4 _returnvalue_2))) (Math|Conversions|ToFloat(Integer) (Math|Integer|%(Integer) _counter _returnvalue)) (Math|Conversions|ToFloat(Integer) _returnvalue_4)) 1e+02)))
    (Math|Integer|IncrementInt (Variables|Default|GetCounter))))

(event EventBeginPlay
  (Utilities|Time|SetTimerbyEvent (delegate Custom|Builder) (/ 1.0 (Variables|Default|GetCubesPerSecond)) true))

(fn ConstructionScript)